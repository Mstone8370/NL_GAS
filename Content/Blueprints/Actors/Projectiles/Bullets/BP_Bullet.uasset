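; Bullet projectile actor that adds a trail effect to whatever behavior its parent class provides.
; On BeginPlay it spawns a separate BP_BulletTrailFX actor and attaches it to the bullet's mesh.
; When destroyed, it detaches the trail in world space and calls BulletHit on it, so the effect is not tied to the destroyed bullet.
; Tick also draws a debug point at the bullet's location.
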(event EventBeginPlay
  (|CallParentFunction)
  (bind _returnvalue (Game|SpawnActorfromClass "/Game/Blueprints/Actors/FX/BP_BulletTrailFX.BP_BulletTrailFX_C" (Math|Transform|MakeTransform "0, 0, 0" "0, 0, 0" "1.000000,1.000000,1.000000") "AlwaysSpawn" "MultiplyWithRoot" 0 0))
  (Transformation|AttachComponentToComponent _returnvalue (Variables|Character|GetMesh) "None" "KeepRelative" "KeepWorld" "KeepWorld" true)
  (Variables|Default|SetBulletTrailFX _returnvalue))

(event EventDestroyed
  (bind _bullettrailfx (Variables|Default|GetBulletTrailFX)
    (:then
      (Transformation|DetachFromActor _bullettrailfx "KeepWorld" "KeepWorld" "KeepWorld")
      (Default|BulletHit _bullettrailfx))
    (:else)))

(event EventTick
  (params (DeltaSeconds :type Float%20%28single-precision%29))
  (Rendering|Debug|DrawDebugPoint (Transformation|GetActorLocation) 2.0 "(R=0.859375,G=0.733282,B=0.000000,A=1.000000)" 0.0))

(fn ConstructionScript)