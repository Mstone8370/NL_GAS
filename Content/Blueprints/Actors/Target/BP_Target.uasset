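; BP_Target is a target actor that reports the damage it takes back to the player who caused it.
; OnTakenDamage feeds HandleDamage, which reads the hit's physical material: PM_Target_NoDamage discards the hit and PM_Target_Center marks it critical.
; The result goes to the NLPlayerController resolved from the source Ability System Component through OnCausedDamage, and the target itself applies no damage.
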(event EventBeginPlay)

(event Collision|EventActorBeginOverlap
  (params (OtherActor :type Actor%20Object%20Reference)))

(event EventTick
  (params (DeltaSeconds :type Float%20%28single-precision%29)))

(event EventOnTakenDamage
  (params (Damage :type Float%20%28single-precision%29) (DamageEffectParams :type Damage%20Effect%20Params%20Structure%20%28by%20ref%29))
  (CallFunction|HandleDamage Damage DamageEffectParams))

(fn ConstructionScript)

(fn HandleDamage
  (params (Damage :type Float%20%28double-precision%29) (InDamageEffectParams :type Damage%20Effect%20Params%20Structure))
  (bind (_damagegameplayeffectclass _sourceasc _targetasc _hitresult) (Utilities|Struct|BreakDamageEffectParams InDamageEffectParams))
  (bind _physmat (Collision|BreakHitResult _hitresult))
  (Utilities|FlowControl|Sequence
    (:then_0
      (Utilities|IsValid _physmat
        (:Is%20Valid
          (if (== _physmat "/Game/Blueprints/Actors/Target/PM_Target_NoDamage.PM_Target_NoDamage")
            (return)
            (else
              (LocalVariables|SetbIsCriticalHit (== _physmat "/Game/Blueprints/Actors/Target/PM_Target_Center.PM_Target_Center")))))))
    (:then_1
      (bind _asnlplayer_controller (Utilities|Casting|CastToNLPlayerController (Class|NLFunctionLibrary|GetAbilitySystemPlayerController _sourceasc)))
      (Class|NLPlayerController|OnCausedDamage _asnlplayer_controller Damage (LocalVariables|GetbIsCriticalHit) self))))