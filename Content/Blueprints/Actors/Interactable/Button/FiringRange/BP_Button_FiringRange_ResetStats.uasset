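; Firing range button that resets the stats of the player who activates it.
; On interaction start, it gets the interactor's BP_NLPlayerState_FiringRange and calls ResetPlayerStats.
; Taking damage while not already interacting also activates it, with the damage source's avatar pawn as interactor.
; That damage-triggered interaction is deferred to the next tick and runs only if the pawn is still valid.
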(event Custom|StartInteractionNextTick
  (bind _pendinginteractor (Variables|Default|GetPendingInteractor)
    (:then
      (Class|Interactable|StartInteraction _pendinginteractor))
    (:else)))

(event EventOnStartInteraction
  (params (Interactor :type Pawn%20Object%20Reference))
  (bind _returnvalue (Class|NLFunctionLibrary|GetPlayerStatefromActor Interactor))
  (|CallParentFunction Interactor)
  (Utilities|IsValid _returnvalue
    (:Is%20Valid
      (bind _asbp_nlplayer_state_firing_range (Utilities|Casting|CastToBP_NLPlayerState_FiringRange _returnvalue))
      (Class|NLPlayerStateFiringRange|ResetPlayerStats _asbp_nlplayer_state_firing_range))))

(event EventOnTakenDamage
  (params (Damage :type Float%20%28single-precision%29) (DamageEffectParams :type Damage%20Effect%20Params%20Structure%20%28by%20ref%29))
  (if (not (Variables|Default|GetbIsInteracting))
    (bind _as폰 (Utilities|Casting|CastToPawn (Class|NLFunctionLibrary|GetAbilitySystemAvatarActor (.SourceASC (Utilities|Struct|BreakDamageEffectParams DamageEffectParams)))))
    (Variables|Default|SetPendingInteractor _as폰)
    (Class|KismetSystemLibrary|SetTimerforNextTickDelegate (delegate Custom|StartInteractionNextTick))))

(fn ConstructionScript
  (|CallParentFunction))