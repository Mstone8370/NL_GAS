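; BP_Button is an interactable button actor with a light that can be switched on and off.
; On BeginPlay it finds the M_Button_light slot on the ButtonPress component and creates a dynamic material instance for it.
; Light_On and Light_Off set the point light intensity and that material's emissive color.
; The interaction start and end events are empty, and an authority-only timer fragment is left unconnected.
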(event Custom|Light_On
  (Rendering|Components|Light|SetIntensity (Variables|Default|GetPointLight) 5e+01)
  (bind _dynamicmaterial_buttonlight (Variables|Default|GetDynamicMaterial_ButtonLight)
    (:then
      (Rendering|Material|SetVectorParameterValue _dynamicmaterial_buttonlight "EmissiveColor" (Variables|Default|GetLightOnColor) :!class /Script/Engine.MaterialInstanceDynamic))
    (:else)))

(event Custom|Light_Off
  (Rendering|Components|Light|SetIntensity (Variables|Default|GetPointLight) 0.0)
  (bind _dynamicmaterial_buttonlight (Variables|Default|GetDynamicMaterial_ButtonLight)
    (:then
      (Rendering|Material|SetVectorParameterValue _dynamicmaterial_buttonlight "EmissiveColor" (Variables|Default|GetLightOffColor) :!class /Script/Engine.MaterialInstanceDynamic))
    (:else)))

(event EventBeginPlay
  (for (_array_element _array_index) (Rendering|Material|GetMaterials (Variables|Default|GetButton_Press))
    (bind _returnvalue (Rendering|Material|GetBaseMaterial _array_element))
    (if (== _returnvalue "/Game/Assets/Interactable/Button/Default/Materials/M_Button_light.M_Button_light")
      (bind _returnvalue_2 (Rendering|Material|CreateDynamicMaterialInstance (Variables|Default|GetButton_Press) _array_index _array_element "None" :!class /Script/Engine.PrimitiveComponent))
      (Variables|Default|SetDynamicMaterial_ButtonLight _returnvalue_2))))

(event EventOnEndInteraction)

(event EventOnStartInteraction
  (params (Interactor :type Pawn%20Object%20Reference)))

(fn ConstructionScript)