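; BP_Spec is a spectator-style pawn that places the local player's view at a random predefined spec point in the level.
; On BeginPlay it picks one BP_SpecPoint actor at random and moves itself to that location.
; If a local viewing player controller exists, it copies the point's rotation to the control rotation and sets look-input ignore from the point's LockView flag.
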(event EventBeginPlay
  (bind _returnvalue (Pawn|GetLocalViewingPlayerController))
  (bind _outactors (Actor|GetAllActorsOfClass "/Game/Blueprints/Actors/BP_SpecPoint.BP_SpecPoint_C"))
  (Variables|Default|SetTargetSpecPoint (.OutItem (Utilities|Array|Random _outactors)))
  (Utilities|IsValid (.OutItem (Utilities|Array|Random _outactors))
    (:Is%20Valid
      (Transformation|SetActorLocation (Transformation|GetActorLocation (Variables|Default|GetTargetSpecPoint)) false false)
      (Utilities|IsValid _returnvalue
        (:Is%20Valid
          (Pawn|SetControlRotation _returnvalue (Transformation|GetActorRotation (Variables|Default|GetTargetSpecPoint)))
          (Input|SetIgnoreLookInput _returnvalue (Variables|/Game/Blueprints/Actors/BP_SpecPoint.BP_SpecPoint_C|GetLockView (Variables|Default|GetTargetSpecPoint))))))))

(event Collision|EventActorBeginOverlap
  (params (OtherActor :type Actor%20Object%20Reference)))

(event EventTick
  (params (DeltaSeconds :type Float%20%28single-precision%29)))

(fn ConstructionScript)