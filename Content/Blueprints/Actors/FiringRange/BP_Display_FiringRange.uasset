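; BP_Display_FiringRange is a firing range display actor that shows a score against a maximum score.
; It exposes SetScore and ClearScore, which forward to the WBP_Display_FiringRange widget held by its Widget component.
; GetWBP casts that component's widget and stores it in a variable before returning it on each call.
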(fn ConstructionScript)

(fn SetScore
  (params (Score :type Integer) (MaxScore :type Integer))
  (Default|SetScore (CallFunction|GetWBP) Score MaxScore))

(fn GetWBP
  (Utilities|FlowControl|Sequence
    (:then_0
      (bind _widget (Variables|Default|GetWidget)
        (:then
          (bind _aswbp_display_firing_range (Utilities|Casting|CastToWBP_Display_FiringRange (UserInterface|GetWidget _widget)))
          (Variables|Default|SetWBP _aswbp_display_firing_range))
        (:else)))
    (:then_1
      (return (Variables|Default|GetWBP)))))

(fn ClearScore
  (Default|ClearScore (CallFunction|GetWBP)))