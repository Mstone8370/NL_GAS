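; Game mode for the firing range, which runs a timed wave of target spawns tied to a registered button.
; RegisterButton stores the button and binds an event to its press.
; Start spawns twenty BP_Target actors at random points within a fixed volume, pausing briefly after each, then ends the button's interaction.
; TODOs note planned pooling, varied spacing and timing, and waiting until all targets are cleared.
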(event Custom|RegisterButton
  (params (Button :type BP%20Button%20Firing%20Range%20Object%20Reference))
  (bind _output_get (Variables|Default|SetButton Button))
  (EventDispatchers|BindEventtoPressed _output_get (EventDispatchers|CreateEvent :!event Custom|Start)))

(event Custom|Start
  (Variables|Default|SetCount 0)
  (if (< (Variables|Default|GetCount) 20) :!label _label
    ;[1 1 1] TODO: 풀을 만들어서 기존 타겟 재사용
    (Game|SpawnActorfromClass "/Game/Blueprints/Actors/Target/BP_Target.BP_Target_C" (Math|Transform|MakeTransform (Math|Vector|MakeVector (Math|Random|RandomFloatinRange -5.5e+02 1.15e+03) (Math|Random|RandomFloatinRange -4.35e+03 -1.35e+03) (Math|Random|RandomFloatinRange 2e+02 6.5e+02))) "Undefined" "MultiplyWithRoot" 0 0)
    (Math|Integer|IncrementInt (Variables|Default|GetCount)
      (:%20%20
        ;[1 1 1] TODO: 처음엔 길게, 나중엔 짧게
        (Utilities|FlowControl|Delay 0.5)
        (goto _label)))
    (else
      ;[1 1 1] TODO: 모든 타겟이 제거된 후에
      (bind _button (Variables|Default|GetButton)
        (:then
          (Class|Interactable|EndInteraction _button))
        (:else)))))

(fn ConstructionScript
  (|CallParentFunction))