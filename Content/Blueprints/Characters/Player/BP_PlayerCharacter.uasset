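; Player character Blueprint that adds local feedback, team visuals and debug input on top of its parent class.
; Team events swap mesh materials for enemy, friendly or neutral, showing the name widget only on friendlies other than self.
; Jumps and landings trigger camera shakes on the locally viewing controller, scaled by vertical speed when landing.
; Tab toggles the player stats widget, Q test-drops the current weapon, and GameMode restart snippets sit unconnected.
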(event Custom|WeaponDropTest
  (Class|NLCharacterComponent|DropCurrentWeapon (Variables|Default|GetNLCharacterComponent)))

(event EventOnJumped
  (bind _returnvalue (Pawn|GetLocalViewingPlayerController))
  (Utilities|IsValid _returnvalue
    (:Is%20Valid
      (Game|Feedback|ClientStartCameraShake _returnvalue "/Game/Blueprints/CameraShake/Locomotion/CS_Jump.CS_Jump_C" 1.0 "CameraLocal" "0, 0, 0"))))

(event EventTick
  (params (DeltaSeconds :type Float%20%28single-precision%29))
  (|CallParentFunction DeltaSeconds))

(event EventOnLanded
  (params (Hit :type Hit%20Result%20Structure%20%28by%20ref%29))
  (bind _returnvalue (Pawn|GetLocalViewingPlayerController))
  (bind _charactermovement (Variables|Character|GetCharacterMovement))
  (bind _returnvalue_2 (Pawn|Components|CharacterMovement|GetLastUpdateVelocity _charactermovement))
  (bind _returnvalue_3 (Math|Float|Absolute(Float) (.z _returnvalue_2)))
  (Utilities|IsValid _returnvalue
    (:Is%20Valid
      (if (> _returnvalue_3 2e+02)
        (Game|Feedback|ClientStartCameraShake _returnvalue (select (>= _returnvalue_3 1e+03) "/Game/Blueprints/CameraShake/Locomotion/CS_Landed_High.CS_Landed_High_C" "/Game/Blueprints/CameraShake/Locomotion/CS_Landed_low.CS_Landed_low_C") 1.0 "CameraLocal" "0, 0, 0")))))

(event EventSetasEnemy
  ;[1 1 1] Team
  (|CallParentFunction)
  (for (_array_element _array_index) (Variables|Team|GetEnemyMaterials)
    (Rendering|Material|SetMaterial (Variables|Character|GetMesh) _array_index _array_element)
    (Rendering|SetVisibility (Variables|Default|GetCharacterNameWidgetComponent) false false)))

(event EventSetasFriendly
  (params (bSelf :type Boolean))
  ;[1 1 1] Team
  (|CallParentFunction bSelf)
  (for (_array_element _array_index) (Variables|Team|GetFriendlyMaterials)
    (Rendering|Material|SetMaterial (Variables|Character|GetMesh) _array_index _array_element)
    (Rendering|SetVisibility (Variables|Default|GetCharacterNameWidgetComponent) (not bSelf) true)))

(event EventOnUserNameSet
  (params (UserName :type String))
  ;[1 1 1] Character name
  (bind _aswbp_user_name (Utilities|Casting|CastToWBP_UserName (UserInterface|GetWidget (Variables|Default|GetCharacterNameWidgetComponent))))
  (Default|SetUserName _aswbp_user_name UserName))

(event EventSetasNeutral
  ;[1 1 1] Team
  (|CallParentFunction)
  (for (_array_element _array_index) (Variables|Team|GetNeutralMaterials)
    (Rendering|Material|SetMaterial (Variables|Character|GetMesh) _array_index _array_element)
    (Rendering|SetVisibility (Variables|Default|GetCharacterNameWidgetComponent) false false)))

(event EventOnCharacterNameWidgetInitialized
  ;[1 1 1] Character name
  (bind _aswbp_user_name (Utilities|Casting|CastToWBP_UserName (UserInterface|GetWidget (Variables|Default|GetCharacterNameWidgetComponent))))
  (Default|SetUserName _aswbp_user_name (Class|NLFunctionLibrary|GetPlayerName self)))

(event Input|KeyboardEvents|Q
  (params (Key :type Key%20Structure :default "None"))
  (:Pressed
    (CallFunction|WeaponDropTest)))

(event Input|KeyboardEvents|T
  (params (Key :type Key%20Structure :default "None"))
  ;[1 1 1] TODO: TEST
)

(event Input|KeyboardEvents|Tab
  (params (Key :type Key%20Structure :default "None"))
  (:Pressed
    (Utilities|FlowControl|FlipFlop
      (:A
        (bind _returnvalue (UserInterface|CreateWidget "/Game/Blueprints/UI/UserWidgets/PlayersStat/WBP_PlayersStat.WBP_PlayersStat_C"))
        (bind _output_get (Variables|Default|SetWBP_PlayersStat _returnvalue))
        (UserInterface|Viewport|AddtoViewport _output_get 0))
      (:B
        (bind _wbp_playersstat (Variables|Default|GetWBP_PlayersStat)
          (:then
            (Default|Clear _wbp_playersstat)
            (Widget|RemovefromParent _wbp_playersstat))
          (:else))))))

(fn ConstructionScript
  (|CallParentFunction))