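; BP_DamageTextWidgetComponent is a damage text widget component that displays a damage value and its critical-hit state through a WBP_DamageText widget.
; It extends parent logic for value updates and the end of the update wait, forwarding the value and critical flag, then the lifetime, to the widget.
; A helper lazily casts and caches the widget reference on first use.
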(event EventOnStopWatingUpdate
  (|CallParentFunction)
  (Default|OnWaitingUpdateFinished (CallFunction|GetDamageTextWidget) (Variables|Default|GetLifeTime)))

(event EventUpdateValue
  (params (InValue :type Float%20%28single-precision%29) (bIsCriticalHit :type Boolean))
  (|CallParentFunction InValue bIsCriticalHit)
  (Default|SetValue (CallFunction|GetDamageTextWidget) (Variables|Default|GetValue) bIsCriticalHit))

(fn GetDamageTextWidget
  (Variables|Default|GetWidget_DamageText
    (:then
      _)
    (:else
      (bind _aswbp_damage_text (Utilities|Casting|CastToWBP_DamageText (UserInterface|GetWidget)))
      (Variables|Default|SetWidget_DamageText _aswbp_damage_text)))
  (return (Variables|Default|GetWidget_DamageText)))