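; HUD that draws a dynamic crosshair and hit indicator for the player's NL character.
; On native init it creates five crosshair widgets and a damage-cause indicator.
; DrawHUD projects the aim point and a spread-rotated direction to get screen center and line offset.
; Tick interpolates that offset, repositions the widgets and fades the four lines out during ADS, while death and respawn handlers toggle crosshair visibility.
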(event EventBeginPlay
  (Variables|Default|SetbCrosshairInitialized false))

(event EventTick
  (params (DeltaSeconds :type Float%20%28single-precision%29))
  (CallFunction|UpdateCrosshair DeltaSeconds))

(event EventDrawHUD
  (params (SizeX :type Integer) (SizeY :type Integer))
  (CallFunction|UpdateCrosshairProperties))

(event EventOnNativeInitialized
  (CallFunction|Initialize))

(fn ConstructionScript)

(fn UpdateCrosshairProperties
  (bind (_outlocation _outrotation) (Class|NLHUD|GetPlayerAimPoint))
  (if (Variables|Default|GetbCrosshairInitialized)
    (Utilities|IsValid (CallFunction|GetControlledNLCharacter)
      (:Is%20Valid
        (bind _returnvalue (Class|PlayerInterface|GetWeaponSpreadValue(Message) (Class|HUD|GetOwningPawn)))
        (LocalVariables|SetSpreadVal _returnvalue)
        (LocalVariables|SetViewLocation _outlocation)
        (LocalVariables|SetCenterDirection (Math|Vector|GetForwardVector _outrotation))
        (Variables|CrosshairProperties|Position|SetCenterPositionX (.x (Class|HUD|Project (+ (LocalVariables|GetCenterDirection) (LocalVariables|GetViewLocation)) true)))
        (Variables|CrosshairProperties|Position|SetCenterPositionY (.y (Class|HUD|Project (+ (LocalVariables|GetCenterDirection) (LocalVariables|GetViewLocation)) true)))
        (Variables|CrosshairProperties|Position|SetSpreadPositionDelta (+ (Math|Float|Absolute(Float) (- (Variables|CrosshairProperties|Position|GetCenterPositionY) (.y (Class|HUD|Project (+ (Math|Vector|RotateVectorAroundAxis (LocalVariables|GetCenterDirection) (* (LocalVariables|GetSpreadVal) 2.0) (Math|Vector|GetRightVector (Pawn|GetControlRotation (Game|Player|GetOwningPlayerController) :!class /Script/Engine.Controller))) (LocalVariables|GetViewLocation)) true)))) (/ (Variables|CrosshairProperties|Size|GetLineLength) 2.0)))))))

(fn GetControlledNLCharacter
  (bind _returnvalue (Game|Player|GetOwningPlayerController))
  (bind _returnvalue_2 (Pawn|GetControlledPawn _returnvalue))
  (Variables|Default|GetControlledNLCharacter
    (:then
      _)
    (:else
      (Utilities|IsValid _returnvalue_2
        (:Is%20Valid
          (bind _asnlplayer_character (Utilities|Casting|CastToNLPlayerCharacter _returnvalue_2))
          (Variables|Default|SetControlledNLCharacter _asnlplayer_character)))))
  (return (Variables|Default|GetControlledNLCharacter)))

(fn SetWidgetPosition
  (params (Widget :type User%20Widget%20Object%20Reference) (PositionX :type Float%20%28double-precision%29) (PositionY :type Float%20%28double-precision%29))
  (Utilities|IsValid Widget
    (:Is%20Valid
      (Class|UserWidget|SetPositioninViewport Widget (Math|Vector2D|MakeVector2D PositionX PositionY) true))))

(fn UpdateCrosshair
  (params (DeltaTime :type Float%20%28double-precision%29))
  (if (Variables|Default|GetbCrosshairInitialized)
    (CallFunction|UpdateCrosshairPosition DeltaTime)
    (CallFunction|UpdateCrosshairAlpha DeltaTime)
    (CallFunction|SetWidgetPosition (Variables|Default|GetWidget_DamageIndicator) (Variables|CrosshairProperties|Position|GetCenterPositionX) (Variables|CrosshairProperties|Position|GetCenterPositionY))))

(fn UpdateCrosshairPosition
  (params (DeltaTime :type Float%20%28double-precision%29))
  (Variables|CrosshairProperties|Position|SetSpredPositionDeltaInterped (Math|Interpolation|FInterpTo (Variables|CrosshairProperties|Position|GetSpredPositionDeltaInterped) (Variables|CrosshairProperties|Position|GetSpreadPositionDelta) DeltaTime (Variables|CrosshairProperties|Position|GetPositionInterpSpeed)))
  (CallFunction|SetWidgetPosition (Variables|Widget_Crosshair|GetCrosshair_Center) (Variables|CrosshairProperties|Position|GetCenterPositionX) (Variables|CrosshairProperties|Position|GetCenterPositionY))
  (CallFunction|SetWidgetPosition (Variables|Widget_Crosshair|GetCrosshair_Up) (Variables|CrosshairProperties|Position|GetCenterPositionX) (- (Variables|CrosshairProperties|Position|GetCenterPositionY) (Variables|CrosshairProperties|Position|GetSpredPositionDeltaInterped)))
  (CallFunction|SetWidgetPosition (Variables|Widget_Crosshair|GetCrosshair_Down) (Variables|CrosshairProperties|Position|GetCenterPositionX) (+ (Variables|CrosshairProperties|Position|GetCenterPositionY) (Variables|CrosshairProperties|Position|GetSpredPositionDeltaInterped)))
  (CallFunction|SetWidgetPosition (Variables|Widget_Crosshair|GetCrosshair_Right) (+ (Variables|CrosshairProperties|Position|GetCenterPositionX) (Variables|CrosshairProperties|Position|GetSpredPositionDeltaInterped)) (Variables|CrosshairProperties|Position|GetCenterPositionY))
  (CallFunction|SetWidgetPosition (Variables|Widget_Crosshair|GetCrosshair_Left) (- (Variables|CrosshairProperties|Position|GetCenterPositionX) (Variables|CrosshairProperties|Position|GetSpredPositionDeltaInterped)) (Variables|CrosshairProperties|Position|GetCenterPositionY)))

(fn UpdateCrosshairAlpha
  (params (DeltaTime :type Float%20%28double-precision%29))
  (Variables|CrosshairProperties|Alpha|SetCrosshairAlphaInterped (Math|Interpolation|FInterpTo (Variables|CrosshairProperties|Alpha|GetCrosshairAlphaInterped) (Math|Float|SelectFloat 0.0 1.0 (Class|NLPlayerCharacter|IsADS (CallFunction|GetControlledNLCharacter))) DeltaTime (Variables|CrosshairProperties|Alpha|GetAlphaInterpSpeed)))
  (Default|SetAlpha (Variables|Widget_Crosshair|GetCrosshair_Up) (Variables|CrosshairProperties|Alpha|GetCrosshairAlphaInterped))
  (Default|SetAlpha (Variables|Widget_Crosshair|GetCrosshair_Down) (Variables|CrosshairProperties|Alpha|GetCrosshairAlphaInterped))
  (Default|SetAlpha (Variables|Widget_Crosshair|GetCrosshair_Right) (Variables|CrosshairProperties|Alpha|GetCrosshairAlphaInterped))
  (Default|SetAlpha (Variables|Widget_Crosshair|GetCrosshair_Left) (Variables|CrosshairProperties|Alpha|GetCrosshairAlphaInterped)))

(fn ShowDamageCauseIndicator
  (params (Damage :type Float%20%28single-precision%29) (bIsCriticalHit :type Boolean) (DamagedActor :type Actor%20Object%20Reference))
  (Utilities|FlowControl|Sequence
    (:then_0
      (Default|OnDamageCaused (Variables|Default|GetWidget_DamageIndicator) bIsCriticalHit))))

(fn Initialize
  (bind _returnvalue (Game|Player|GetOwningPlayerController))
  (bind _centerdotsize (Variables|CrosshairProperties|Size|GetCenterDotSize))
  (if (Variables|Default|GetbCrosshairInitialized)
    (Development|PrintString "Already Initialized")
    (else
      (Utilities|FlowControl|Sequence
        (:then_0
          (Utilities|FlowControl|Sequence
            (:then_0
              (bind _returnvalue_2 (UserInterface|CreateWidget "/Game/Blueprints/UI/UserWidgets/HUD/WBP_Crosshair.WBP_Crosshair_C" _returnvalue _centerdotsize _centerdotsize (Variables|CrosshairProperties|Size|GetOutlineThickness)))
              (bind _output_get (Variables|Widget_Crosshair|SetCrosshair_Center _returnvalue_2))
              (UserInterface|Viewport|AddtoViewport _output_get 0))
            (:then_1
              (bind _returnvalue_3 (UserInterface|CreateWidget "/Game/Blueprints/UI/UserWidgets/HUD/WBP_Crosshair.WBP_Crosshair_C" _returnvalue (Variables|CrosshairProperties|Size|GetLineThickness) (Variables|CrosshairProperties|Size|GetLineLength) (Variables|CrosshairProperties|Size|GetOutlineThickness)))
              (bind _output_get_2 (Variables|Widget_Crosshair|SetCrosshair_Up _returnvalue_3))
              (UserInterface|Viewport|AddtoViewport _output_get_2 0))
            (:then_2
              (bind _returnvalue_4 (UserInterface|CreateWidget "/Game/Blueprints/UI/UserWidgets/HUD/WBP_Crosshair.WBP_Crosshair_C" _returnvalue (Variables|CrosshairProperties|Size|GetLineThickness) (Variables|CrosshairProperties|Size|GetLineLength) (Variables|CrosshairProperties|Size|GetOutlineThickness)))
              (bind _output_get_3 (Variables|Widget_Crosshair|SetCrosshair_Down _returnvalue_4))
              (UserInterface|Viewport|AddtoViewport _output_get_3 0))
            (:then_3
              (bind _returnvalue_5 (UserInterface|CreateWidget "/Game/Blueprints/UI/UserWidgets/HUD/WBP_Crosshair.WBP_Crosshair_C" _returnvalue (Variables|CrosshairProperties|Size|GetLineLength) (Variables|CrosshairProperties|Size|GetLineThickness) (Variables|CrosshairProperties|Size|GetOutlineThickness)))
              (bind _output_get_4 (Variables|Widget_Crosshair|SetCrosshair_Right _returnvalue_5))
              (UserInterface|Viewport|AddtoViewport _output_get_4 0))
            (:then_4
              (bind _returnvalue_6 (UserInterface|CreateWidget "/Game/Blueprints/UI/UserWidgets/HUD/WBP_Crosshair.WBP_Crosshair_C" _returnvalue (Variables|CrosshairProperties|Size|GetLineLength) (Variables|CrosshairProperties|Size|GetLineThickness) (Variables|CrosshairProperties|Size|GetOutlineThickness)))
              (bind _output_get_5 (Variables|Widget_Crosshair|SetCrosshair_Left _returnvalue_6))
              (UserInterface|Viewport|AddtoViewport _output_get_5 0))))
        (:then_1
          (bind _returnvalue_7 (UserInterface|CreateWidget "/Game/Blueprints/UI/UserWidgets/HUD/WBP_DamageCauseIndicator.WBP_DamageCauseIndicator_C" (Game|Player|GetOwningPlayerController)))
          (bind _output_get_6 (Variables|Default|SetWidget_DamageIndicator _returnvalue_7))
          (UserInterface|Viewport|AddtoViewport _output_get_6 0))
        (:then_2
          (Variables|Default|SetbCrosshairInitialized true))))))

(fn OnCharacterDead
  (CallFunction|SetCrosshairVisibility "Hidden"))

(fn SetCrosshairVisibility
  (params (InVisibility :type ESlateVisibility%20Enum :default "Visible"))
  (Widget|SetVisibility (Variables|Widget_Crosshair|GetCrosshair_Center) InVisibility))

(fn OnCharacterRespawn
  (CallFunction|SetCrosshairVisibility "HitTestInvisible"))