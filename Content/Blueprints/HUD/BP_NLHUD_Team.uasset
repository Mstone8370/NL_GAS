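; Team HUD Blueprint that keeps the overlay and crosshair hidden until a round begins.
; On initialization it hides both and subscribes to the overlay widget controller's round-started event.
; That event shows a round-wait countdown widget and starts a one-shot timer for the wait time.
; OnRoundBegin, presumably the timer's callback, reveals overlay and crosshair, removes the wait widget and broadcasts the controller's initial values.
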(event Custom|OnRoundStarted_Event
  (params (WaitTime :type Integer))
  (bind _returnvalue (Math|Conversions|ToFloat(Integer) WaitTime))
  (bind _returnvalue_2 (UserInterface|CreateWidget (Variables|Default|GetRoundWaitWidgetClass)))
  (bind _output_get (Variables|Default|SetRoundWaitWidgetObject _returnvalue_2))
  (Default|SetTimer _output_get _returnvalue)
  (UserInterface|Viewport|AddtoViewport (Variables|Default|GetRoundWaitWidgetObject) 0)
  (Utilities|Time|SetTimerbyEvent (EventDispatchers|CreateEvent :!event OnRoundBegin) _returnvalue))

(event EventOnNativeInitialized
  (|CallParentFunction)
  (Widget|SetVisibility (Variables|Default|GetOverlayWidget) "Hidden")
  (CallFunction|SetCrosshairVisibility "Hidden")
  (bind _overlaywidgetcontroller (Variables|Default|GetOverlayWidgetController)
    (:then
      (EventDispatchers|AssignOnRoundStarted _overlaywidgetcontroller (delegate Custom|OnRoundStarted_Event)))
    (:else)))

(fn ConstructionScript
  (|CallParentFunction))

(fn OnRoundBegin
  (Widget|SetVisibility (Variables|Default|GetOverlayWidget) "HitTestInvisible")
  (CallFunction|SetCrosshairVisibility "HitTestInvisible")
  (Widget|RemovefromParent (Variables|Default|GetRoundWaitWidgetObject))
  (Class|NLWidgetController|BroadcastInitialValues (Variables|Default|GetOverlayWidgetController)))