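; GA_Test is a test gameplay ability that fires a BP_TestProjectile along a targeting trace.
; An instant WaitTargetData task runs a debug single-line trace starting at the local player's viewpoint, or the avatar's location without one.
; On valid data, only the authority spawns the projectile slightly ahead of the trace start, facing the impact point or trace end.
; Valid and cancelled results print debug strings, and the ability ends after a short delay.
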(event Ability|EventActivateAbility
  (bind _returnvalue (Ability|GetAvatarActorfromActorInfo))
  (bind _as캐릭터 (Utilities|Casting|CastToCharacter (Ability|GetAvatarActorfromActorInfo))
    (:then
      (Variables|Default|SetPC (Pawn|GetLocalViewingPlayerController _as캐릭터)))
    (:CastFailed
      _))
  (bind _data (|WaitTargetData :ConfirmationType "Instant" :Class "/Script/GameplayAbilities.GameplayAbilityTargetActor_SingleLineTrace" :TraceProfile "(Name=\"BlockAll\")" :StartLocation (Utilities|Struct|MakeGameplayAbilityTargetingLocationInfo "LiteralTransform" (Math|Transform|MakeTransform (Math|Vector|SelectVector (.Location (Pawn|GetPlayerViewPoint (Variables|Default|GetPC))) (Transformation|GetActorLocation _returnvalue) (Utilities|IsValid (Variables|Default|GetPC))) (Transformation|GetActorRotation _returnvalue))) :ReticleClass "/Script/GameplayAbilities.GameplayAbilityWorldReticle" :bDebug true)
    (:ValidData
      (Development|PrintString "ValidData")
      (Ability|HasAuthority
        (:True
          (Game|SpawnActorfromClass "/Game/Blueprints/AbilitySystem/Abilities/Test/BP_TestProjectile.BP_TestProjectile_C" (Math|Transform|MakeTransform (+ (* (Math|Vector|Normalize (- (Math|Vector|SelectVector (.ImpactPoint (Collision|BreakHitResult (Ability|TargetData|GetHitResultfromTargetData _data))) (.TraceEnd (Collision|BreakHitResult (Ability|TargetData|GetHitResultfromTargetData _data))) (.bBlockingHit (Collision|BreakHitResult (Ability|TargetData|GetHitResultfromTargetData _data)))) (.TraceStart (Collision|BreakHitResult (Ability|TargetData|GetHitResultfromTargetData _data))))) 1e+02) (.TraceStart (Collision|BreakHitResult (Ability|TargetData|GetHitResultfromTargetData _data)))) (Math|Rotator|MakeRotfromX (Math|Vector|Normalize (- (Math|Vector|SelectVector (.ImpactPoint (Collision|BreakHitResult (Ability|TargetData|GetHitResultfromTargetData _data))) (.TraceEnd (Collision|BreakHitResult (Ability|TargetData|GetHitResultfromTargetData _data))) (.bBlockingHit (Collision|BreakHitResult (Ability|TargetData|GetHitResultfromTargetData _data)))) (.TraceStart (Collision|BreakHitResult (Ability|TargetData|GetHitResultfromTargetData _data))))))) "AlwaysSpawn" "MultiplyWithRoot" 0 0))
        (:False
          _)))
    (:Cancelled
      (Development|PrintString "Cancelled")))
  (Utilities|FlowControl|Delay 0.1)
  (Ability|EndAbility))