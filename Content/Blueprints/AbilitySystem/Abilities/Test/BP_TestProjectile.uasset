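; Test projectile for the ability system that carries a bullet trail and reacts to impacts differently by network role.
; BeginPlay spawns a trail actor attached to the mesh, and Tick draws a debug point at the projectile's location.
; On sphere hit, the authority destroys the projectile while remotes spawn a Niagara impact effect oriented by the hit normal.
; On destruction, the trail is detached and notified through BulletHit.
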(event OnComponentHit(Sphere)
  (params (HitComponent :type Primitive%20Component%20Object%20Reference) (OtherActor :type Actor%20Object%20Reference) (OtherComp :type Primitive%20Component%20Object%20Reference) (NormalImpulse :type Vector :default "0, 0, 0") (Hit :type Hit%20Result%20Structure%20%28by%20ref%29))
  (bind (_bblockinghit _binitialoverlap _time _distance _location _impactpoint _normal _impactnormal) (Collision|BreakHitResult Hit))
  (Networking|SwitchHasAuthority
    (:Authority
      (Actor|DestroyActor))
    (:Remote
      (bind _returnvalue (Class|NiagaraFunctionLibrary|SpawnSystematLocationwithParams (Utilities|Struct|MakeFXSystemSpawnParameters OtherActor "/Game/Assets/FX/NS_BulletHit.NS_BulletHit" _impactpoint "0.000000,0.000000,0.000000" "1.000000,1.000000,1.000000" 0 "None" "KeepWorldPosition" true true)))
      (Effects|Components|ParticleSystem|SetVectorParameter _returnvalue "Direction" _impactnormal))))

(event EventBeginPlay
  (bind _returnvalue (Game|SpawnActorfromClass "/Game/Blueprints/AbilitySystem/Abilities/Test/BP_BulletTrailFX.BP_BulletTrailFX_C" (Transformation|GetActorTransform) "AlwaysSpawn" "MultiplyWithRoot" 0 0))
  (Transformation|AttachComponentToComponent _returnvalue (Variables|Default|GetStaticMesh) "None" "SnapToTarget" "KeepWorld" "KeepWorld" true)
  (Variables|Default|SetBulletTrailFX _returnvalue))

(event EventTick
  (params (DeltaSeconds :type Float%20%28single-precision%29))
  (Rendering|Debug|DrawDebugPoint (Transformation|GetActorLocation) 2.0 "(R=0.859375,G=0.733282,B=0.000000,A=1.000000)" 0.0))

(event EventDestroyed
  (bind _bullettrailfx (Variables|Default|GetBulletTrailFX)
    (:then
      (Transformation|DetachFromActor _bullettrailfx "KeepWorld" "KeepWorld" "KeepWorld")
      (Default|BulletHit _bullettrailfx))
    (:else)))

(fn ConstructionScript)