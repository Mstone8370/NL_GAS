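; Gameplay ability that handles weapon reloading on the avatar actor.
; Activation is gated by the avatar's StartReloadMessage result, then a replicated loose Ability.Weapon.Reload tag is held until the ability ends.
; Event.Reload gameplay events, child tags included, are forwarded to the avatar as reload state changes.
; Only the authority ends the ability, upon the Finished event.
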(event Ability|EventActivateAbility
  (Ability|GameplayEffect|AddLooseGameplayTags (Ability|GetAvatarActorfromActorInfo) (GameplayTags|MakeGameplayTagContainerfromTag "(TagName=\"Ability.Weapon.Reload\")") true)
  (bind _payload (Ability|Tasks|WaitGameplayEvent "(TagName=\"Event.Reload\")" 0 false false)
    (:EventReceived
      (Class|PlayerInterface|OnWeaponReloadStateChanged(Message) (Ability|GetAvatarActorfromActorInfo) (GameplayTags|MakeLiteralGameplayTag) (.EventTag (Utilities|Struct|BreakGameplayEventData _payload)))
      (if (== (.EventTag (Utilities|Struct|BreakGameplayEventData _payload)) "(TagName=\"Event.Reload.Finished\")")
        (Ability|HasAuthority
          (:True
            (Ability|EndAbility)))))))

(event Ability|EventOnEndAbility
  (params (bWasCancelled :type Boolean))
  (Ability|GameplayEffect|RemoveLooseGameplayTags (Ability|GetAvatarActorfromActorInfo) (GameplayTags|MakeGameplayTagContainerfromTag "(TagName=\"Ability.Weapon.Reload\")") true))

(fn K2CanActivateAbility
  (params (ActorInfo :type Gameplay%20Ability%20Actor%20Info%20Structure) (Handle :type Gameplay%20Ability%20Spec%20Handle%20Structure))
  (bind _returnvalue (Class|PlayerInterface|StartReload(Message) (Ability|GetAvatarActorfromActorInfo)))
  (return "" _returnvalue))