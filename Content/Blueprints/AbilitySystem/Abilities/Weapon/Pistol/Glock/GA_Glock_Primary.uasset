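; Gameplay ability for the Glock's primary fire, still carrying debug prints and a test projectile.
; An instant single-line-trace target data task starts at the local view point, or actor location without a controller, using actor rotation.
; Valid data plays first-person arm and weapon montages, then the authority spawns the projectile slightly ahead, aimed at the impact or trace end.
; The ability ends after a short delay, also when cancelled.
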(event Ability|EventActivateAbility
  (bind _returnvalue (Ability|GetAvatarActorfromActorInfo))
  (bind _as캐릭터 (Utilities|Casting|CastToCharacter (Ability|GetAvatarActorfromActorInfo))
    (:then
      (Variables|Default|SetPC (Pawn|GetLocalViewingPlayerController _as캐릭터)))
    (:CastFailed
      _))
  (bind _data (|WaitTargetData :ConfirmationType "Instant" :Class "/Script/GameplayAbilities.GameplayAbilityTargetActor_SingleLineTrace" :TraceProfile "(Name=\"BlockAll\")" :StartLocation (Utilities|Struct|MakeGameplayAbilityTargetingLocationInfo "LiteralTransform" (Math|Transform|MakeTransform (Math|Vector|SelectVector (.Location (Pawn|GetPlayerViewPoint (Variables|Default|GetPC))) (Transformation|GetActorLocation _returnvalue) (Utilities|IsValid (Variables|Default|GetPC))) (Transformation|GetActorRotation _returnvalue))) :ReticleClass "/Script/GameplayAbilities.GameplayAbilityWorldReticle" :bDebug true)
    (:ValidData
      (bind _asbp_player_character (Utilities|Casting|CastToBP_PlayerCharacter (Ability|GetAvatarActorfromActorInfo))
        (:then
          (Animation|Montage|PlayMontage (Variables|/Script/NL_GAS.NLPlayerCharacter|GetArmMesh _asbp_player_character) "/Game/Assets/Characters/FirstPerson/Arms/Animations/Pistol/Glock/AM_Arms_pov_Glk_hip_fire_additive.AM_Arms_pov_Glk_hip_fire_additive"
            (:then
              (Animation|Montage|PlayMontage (Variables|/Script/NL_GAS.NLPlayerCharacter|GetViewWeaponMesh _asbp_player_character) "/Game/Assets/Weapon/Pistol/Glock/Animations/AM_Glk_fire.AM_Glk_fire"
                (:then
                  _)))))
        (:CastFailed
          _))
      (Development|PrintString "ValidData")
      (Ability|HasAuthority
        (:True
          (Game|SpawnActorfromClass "/Game/Blueprints/AbilitySystem/Abilities/Test/BP_TestProjectile.BP_TestProjectile_C" (Math|Transform|MakeTransform (+ (* (Math|Vector|Normalize (- (Math|Vector|SelectVector (.ImpactPoint (Collision|BreakHitResult (Ability|TargetData|GetHitResultfromTargetData _data))) (.TraceEnd (Collision|BreakHitResult (Ability|TargetData|GetHitResultfromTargetData _data))) (.bBlockingHit (Collision|BreakHitResult (Ability|TargetData|GetHitResultfromTargetData _data)))) (.TraceStart (Collision|BreakHitResult (Ability|TargetData|GetHitResultfromTargetData _data))))) 1e+02) (.TraceStart (Collision|BreakHitResult (Ability|TargetData|GetHitResultfromTargetData _data)))) (Math|Rotator|MakeRotfromX (Math|Vector|Normalize (- (Math|Vector|SelectVector (.ImpactPoint (Collision|BreakHitResult (Ability|TargetData|GetHitResultfromTargetData _data))) (.TraceEnd (Collision|BreakHitResult (Ability|TargetData|GetHitResultfromTargetData _data))) (.bBlockingHit (Collision|BreakHitResult (Ability|TargetData|GetHitResultfromTargetData _data)))) (.TraceStart (Collision|BreakHitResult (Ability|TargetData|GetHitResultfromTargetData _data))))))) "AlwaysSpawn" "MultiplyWithRoot" 0 0))
        (:False
          _)))
    (:Cancelled
      (Development|PrintString "Cancelled")))
  (Utilities|FlowControl|Delay 0.1)
  (Ability|EndAbility))