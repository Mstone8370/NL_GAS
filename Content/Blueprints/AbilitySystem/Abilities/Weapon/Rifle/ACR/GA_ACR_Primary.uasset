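; Primary fire ability for the ACR rifle, firing one shot per activation once the weapon cost commits, otherwise cancelling.
; An instant weapon-trace target gives the aim, and the avatar plays an ADS or normal fire montage.
; Authority spawns a test projectile just ahead of the trace start, aimed at the hit point or trace end, while non-authority adds camera shake and recoil.
; The ability ends after a brief delay.
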(event Ability|EventActivateAbility
  (bind _as_bp_player_character (Variables|Default|GetAs%20BP%20Player%20Character)
    (:then
      _)
    (:else
      (bind _asbp_player_character (Utilities|Casting|CastToBP_PlayerCharacter (Ability|GetAvatarActorfromActorInfo)))
      (Variables|Default|SetAs%20BP%20Player%20Character _asbp_player_character)))
  (bind _returnvalue (Class|NLCharacterComponent|CommitWeaponCost (Variables|/Script/NL_GAS.NLCharacterBase|GetNLCharacterComponent _as_bp_player_character)))
  (if _returnvalue
    (bind _data (|WaitTargetData :ConfirmationType "Instant" :Class "/Script/NL_GAS.TargetActor_WeaponTrace" :TraceProfile "(Name=\"NoCollision\")" :StartLocation (Utilities|Struct|MakeGameplayAbilityTargetingLocationInfo "LiteralTransform" "0.000000,0.000000,0.000000|0.000000,0.000000,-0.000000|1.000000,1.000000,1.000000" (Ability|GetAvatarActorfromActorInfo)) :ReticleClass 0)
      (:ValidData
        (Development|PrintString "ValidData")
        (Class|PlayerInterface|PlayCurrentWeaponMontage(Message) (Ability|GetAvatarActorfromActorInfo) (select (Variables|/Game/Blueprints/Characters/Player/BP_PlayerCharacter.BP_PlayerCharacter_C|GetIsADS_BP (Variables|Default|GetAs%20BP%20Player%20Character)) (GameplayTags|MakeLiteralGameplayTag "(TagName=\"Montage.Weapon.FireADS\")") (GameplayTags|MakeLiteralGameplayTag "(TagName=\"Montage.Weapon.Primary\")")))
        (Ability|HasAuthority
          (:True
            (Game|SpawnActorfromClass "/Game/Blueprints/AbilitySystem/Abilities/Test/BP_TestProjectile.BP_TestProjectile_C" (Math|Transform|MakeTransform (+ (* (Math|Vector|Normalize (- (Math|Vector|SelectVector (.ImpactPoint (Collision|BreakHitResult (Ability|TargetData|GetHitResultfromTargetData _data))) (.TraceEnd (Collision|BreakHitResult (Ability|TargetData|GetHitResultfromTargetData _data))) (.bBlockingHit (Collision|BreakHitResult (Ability|TargetData|GetHitResultfromTargetData _data)))) (.TraceStart (Collision|BreakHitResult (Ability|TargetData|GetHitResultfromTargetData _data))))) 2e+01) (.TraceStart (Collision|BreakHitResult (Ability|TargetData|GetHitResultfromTargetData _data)))) (Math|Rotator|MakeRotfromX (Math|Vector|Normalize (- (Math|Vector|SelectVector (.ImpactPoint (Collision|BreakHitResult (Ability|TargetData|GetHitResultfromTargetData _data))) (.TraceEnd (Collision|BreakHitResult (Ability|TargetData|GetHitResultfromTargetData _data))) (.bBlockingHit (Collision|BreakHitResult (Ability|TargetData|GetHitResultfromTargetData _data)))) (.TraceStart (Collision|BreakHitResult (Ability|TargetData|GetHitResultfromTargetData _data))))))) "AlwaysSpawn" "MultiplyWithRoot" 0 0))
          (:False
            (Camera|PlayWorldCameraShake "/Game/Blueprints/CameraShake/Weapon/Rifle/CS_ACR_Fire.CS_ACR_Fire_C" (Transformation|GetActorLocation (Ability|GetAvatarActorfromActorInfo)) 0.0 1e+02)
            (Class|ControlShakeManager|AddShake (Variables|/Script/NL_GAS.NLPlayerCharacter|GetControlShakeManager (Variables|Default|GetAs%20BP%20Player%20Character)) (Utilities|Struct|MakeControlShakeParams 0.4 "/Game/Blueprints/Data/Recoil.Recoil" "0.500000,0.000000,0.000000"))))
        (Utilities|FlowControl|Delay 0.1)
        (Ability|EndAbility))
      (:Cancelled
        (Development|PrintString "Cancelled" :!label _label)
        (Ability|CancelAbility)))
    (else
      (goto _label))))