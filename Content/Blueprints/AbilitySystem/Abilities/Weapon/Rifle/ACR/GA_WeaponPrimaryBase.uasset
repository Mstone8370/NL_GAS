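; Base gameplay ability for a weapon's primary fire, supporting automatic and burst modes with empty Fire and SpawnFX hooks, presumably for subclasses.
; Each shot commits weapon cost, gets a hit from an instant WaitTargetData trace, then calls Fire, notifies the avatar, plays montages and spawns FX.
; Bursts loop on a delay, while a fire-rate timer is started on activation; non-automatic modes without auto-burst wait for input release before ending.
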(event Custom|OnFireFinished
  (if (or (Utilities|Enum|Equal(Enum) (Variables|Default|GetFireType) "Automatic") (and (Utilities|Enum|Equal(Enum) (Variables|Default|GetFireType) "Burst") (Variables|Weapon|Burst|GetAutoBurst)))
    (Ability|EndAbility)
    (else
      (Ability|Tasks|WaitInputRelease true
        (:OnRelease
          (Ability|EndAbility))))))

(event Ability|EventActivateAbility
  (Variables|Default|SetFireLoopCurrentIdx 0)
  (Variables|Default|SetFireLoopLastIdx (Math|Integer|SelectInt (Variables|Default|GetBurstFireNum) 1 (Utilities|Enum|Equal(Enum) (Variables|Default|GetFireType) "Burst")))
  (Utilities|Time|SetTimerbyEvent (EventDispatchers|CreateEvent :!event Custom|OnFireFinished) (/ (Math|Float|MakeLiteralFloat 1.0) (Variables|Default|GetFirePerSecond)))
  (if (< (Variables|Default|GetFireLoopCurrentIdx) (Variables|Default|GetFireLoopLastIdx)) :!label _label
    (bind (_bislast _returnvalue) (Class|PlayerInterface|CommitWeaponCost(Message) (Ability|GetAvatarActorfromActorInfo)))
    (Variables|Default|SetbIsLastFire _bislast)
    (if _returnvalue
      (bind _data (|WaitTargetData :ConfirmationType "Instant" :Class "/Script/NL_GAS.TargetActor_WeaponTrace" :MaxRange (Variables|Weapon|GetTargetDataMaxRange) :TraceProfile "(Name=\"NoCollision\")" :StartLocation (Utilities|Struct|MakeGameplayAbilityTargetingLocationInfo "LiteralTransform" "0.000000,0.000000,0.000000|0.000000,0.000000,-0.000000|1.000000,1.000000,1.000000" (Ability|GetAvatarActorfromActorInfo)) :ReticleClass 0)
        (:ValidData
          (bind _output_get (Variables|Default|SetTargetDataHitResult (Ability|TargetData|GetHitResultfromTargetData _data)))
          (CallFunction|Fire _output_get)
          (Class|PlayerInterface|WeaponFired(Message) (Ability|GetAvatarActorfromActorInfo) (Variables|Weapon|GetCameraShake))
          (Utilities|FlowControl|Sequence
            (:then_0
              ;[1 1 1] Play ViewModel AnimMontage
              (Class|PlayerInterface|PlayCurrentWeaponMontage(Message) (Ability|GetAvatarActorfromActorInfo) (select (GameplayTags|HasMatchingGameplayTag (Ability|GetAbilitySystemComponentfromActorInfo) "(TagName=\"Ability.Weapon.Secondary\")") (GameplayTags|MakeLiteralGameplayTag "(TagName=\"Montage.Weapon.FireADS\")") (GameplayTags|MakeLiteralGameplayTag "(TagName=\"Montage.Weapon.Primary\")")))
              (if (Variables|Default|GetbIsLastFire)
                (Class|PlayerInterface|PlayCurrentWeaponMontage(Message) (Ability|GetAvatarActorfromActorInfo) (GameplayTags|MakeLiteralGameplayTag "(TagName=\"Montage.Weapon.LastFire\")"))))
            (:then_1
              (CallFunction|SpawnFX (Variables|Default|GetTargetDataHitResult)))
            (:then_2
              (Math|Integer|IncrementInt (Variables|Default|GetFireLoopCurrentIdx)
                (:%20%20
                  (if (Utilities|Enum|Equal(Enum) (Variables|Default|GetFireType) "Burst")
                    (Utilities|FlowControl|Delay (/ (Math|Float|MakeLiteralFloat 1.0) (Variables|Default|GetBurstFirePerSecond)))
                    (goto _label)))))))
        (:Cancelled
          (Ability|CancelAbility :!label _label_2)))
      (else
        (Ability|Tasks|WaitInputRelease false
          (:OnRelease
            (goto _label_2)))))))

(fn Fire
  (params (HitResult :type Hit%20Result%20Structure))
  (return))

(fn SpawnFX
  (params (TargetDataHitResult :type Hit%20Result%20Structure))
  (return))