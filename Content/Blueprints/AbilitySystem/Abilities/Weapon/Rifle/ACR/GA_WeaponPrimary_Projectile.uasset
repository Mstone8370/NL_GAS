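; Gameplay ability for the ACR rifle's primary attack that fires a projectile, currently BP_TestProjectile.
; Fire takes a HitResult and aims from the trace start toward the impact point, or the trace end when nothing blocks.
; It spawns the projectile just ahead of the start along that direction, owned by the avatar actor.
; The authority check does not gate the spawn, and activation logic is left to the parent class.
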(event Ability|EventActivateAbility
  (|CallParentFunction) ; 지금 이 노드는 비활성 상태입니다. \n핀을 끌어서 다른 노드를 연결하면 활성화됩니다.
)

(fn Fire
  (params (HitResult :type Hit%20Result%20Structure))
  (bind (_bblockinghit _binitialoverlap _time _distance _location _impactpoint _normal _impactnormal _physmat _hitactor _hitcomponent _hitbonename _bonename _hititem _elementindex _faceindex _tracestart _traceend) (Collision|BreakHitResult HitResult))
  (Utilities|FlowControl|Sequence
    (:then_0
      (LocalVariables|SetBulletStart _tracestart)
      (LocalVariables|SetBulletEnd (Math|Vector|SelectVector _impactpoint _traceend _bblockinghit))
      (LocalVariables|SetBulletDirection (Math|Vector|Normalize (- (LocalVariables|GetBulletEnd) (LocalVariables|GetBulletStart)))))
    (:then_1
      (Ability|HasAuthority
        (:True
          _)
        (:False
          _))
      (Game|SpawnActorfromClass "/Game/Blueprints/AbilitySystem/Abilities/Test/BP_TestProjectile.BP_TestProjectile_C" (Math|Transform|MakeTransform (+ (* (LocalVariables|GetBulletDirection) 1.0) (LocalVariables|GetBulletStart)) (Math|Rotator|MakeRotfromX (LocalVariables|GetBulletDirection))) "AlwaysSpawn" "MultiplyWithRoot" (Ability|GetAvatarActorfromActorInfo) 0))))