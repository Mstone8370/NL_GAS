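; Gameplay ability for the ACR rifle's single-shot primary fire, firing one shot per activation.
; It commits weapon cost through the avatar, gathers instant target data with a weapon trace target actor, then calls Fire, flagging whether the shot is the last.
; A 0.1-second delay after firing precedes waiting for input release to end the ability.
; When the cost cannot be committed, it waits for release and cancels.
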(event Ability|EventActivateAbility
  (Variables|Default|GetAs%20BP%20Player%20Character
    (:then
      _)
    (:else
      (bind _asbp_player_character (Utilities|Casting|CastToBP_PlayerCharacter (Ability|GetAvatarActorfromActorInfo)))
      (Variables|Default|SetAs%20BP%20Player%20Character _asbp_player_character)))
  (bind (_bislast _returnvalue) (Class|PlayerInterface|CommitWeaponCost(Message) (Ability|GetAvatarActorfromActorInfo)))
  (if _returnvalue
    (bind _data (|WaitTargetData :ConfirmationType "Instant" :Class "/Script/NL_GAS.TargetActor_WeaponTrace" :TraceProfile "(Name=\"NoCollision\")" :StartLocation (Utilities|Struct|MakeGameplayAbilityTargetingLocationInfo "LiteralTransform" "0.000000,0.000000,0.000000|0.000000,0.000000,-0.000000|1.000000,1.000000,1.000000" (Ability|GetAvatarActorfromActorInfo)) :ReticleClass 0)
      (:ValidData
        (CallFunction|Fire _data _bislast)
        (Utilities|FlowControl|Delay 0.1)
        (Ability|Tasks|WaitInputRelease true
          (:OnRelease
            (Ability|EndAbility))))
      (:Cancelled
        (Ability|CancelAbility)))
    (else
      (Ability|Tasks|WaitInputRelease false
        (:OnRelease
          (Ability|CancelAbility))))))