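; Gameplay ability that toggles weapon aim-down-sights by adding or removing the replicated loose tag Ability.Weapon.Secondary on the avatar at each activation.
; It stays active like a passive, waiting for input release and then the next press to end itself, with that press also reactivating it to flip the tag.
; Cancellation clears the tag, while a normal end preserves it, a workaround the author notes as inelegant but working.
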(event Ability|EventActivateAbility
  ;[0.8594 0.7333 0] 좋은 방법은 아닌데 의도대로 작동하긴 함. 이 방식으로는 이 어빌리티가 캔슬되기 전까진 항상 Activate되어있는 상태임. InputPress 이벤트가 들어오면 End되고 바로 Activate되면서 패시브 어빌리티와 유사한 방식으로 작동함.
  (Utilities|FlowControl|Sequence
    (:then_0
      (if (GameplayTags|HasMatchingGameplayTag (Ability|GetAbilitySystemComponentfromActorInfo) "(TagName=\"Ability.Weapon.Secondary\")")
        (Ability|GameplayEffect|RemoveLooseGameplayTags (Ability|GetAvatarActorfromActorInfo) (GameplayTags|MakeLiteralGameplayTagContainer "(GameplayTags=((TagName=\"Ability.Weapon.Secondary\")))") true)
        (else
          (Ability|GameplayEffect|AddLooseGameplayTags (Ability|GetAvatarActorfromActorInfo) (GameplayTags|MakeLiteralGameplayTagContainer "(GameplayTags=((TagName=\"Ability.Weapon.Secondary\")))") true))))
    (:then_1
      (Ability|Tasks|WaitInputRelease true
        (:OnRelease
          (Ability|Tasks|WaitInputPress false
            (:OnPress
              (Ability|EndAbility))))))))

(event Ability|EventOnEndAbility
  (params (bWasCancelled :type Boolean))
  ;[0.8594 0.7333 0] 좋은 방법은 아닌데 의도대로 작동하긴 함. 이 방식으로는 이 어빌리티가 캔슬되기 전까진 항상 Activate되어있는 상태임. InputPress 이벤트가 들어오면 End되고 바로 Activate되면서 패시브 어빌리티와 유사한 방식으로 작동함.
  (if (and bWasCancelled (GameplayTags|HasMatchingGameplayTag (Ability|GetAbilitySystemComponentfromActorInfo) "(TagName=\"Ability.Weapon.Secondary\")"))
    (Ability|GameplayEffect|RemoveLooseGameplayTags (Ability|GetAvatarActorfromActorInfo) (GameplayTags|MakeLiteralGameplayTagContainer "(GameplayTags=((TagName=\"Ability.Weapon.Secondary\")))") true)))