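; Gameplay ability for the player's primary weapon fire, named as an old version.
; It commits weapon cost, takes an instant weapon-trace target, fires, then ends after a short delay; failed commits cancel on input release.
; Fire plays hip or ADS montages, plus a last-shot montage.
; Authority spawns a test projectile along the aim direction, while non-authority instances send a camera-shake message and spawn view-weapon trail and smoke effects.
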(event Ability|EventActivateAbility
  (Variables|Default|GetAs%20BP%20Player%20Character
    (:then
      _)
    (:else
      (bind _asbp_player_character (Utilities|Casting|CastToBP_PlayerCharacter (Ability|GetAvatarActorfromActorInfo)))
      (Variables|Default|SetAs%20BP%20Player%20Character _asbp_player_character)))
  (bind (_bislast _returnvalue) (Class|PlayerInterface|CommitWeaponCost(Message) (Ability|GetAvatarActorfromActorInfo)))
  (if _returnvalue
    (bind _data (|WaitTargetData :ConfirmationType "Instant" :Class "/Script/NL_GAS.TargetActor_WeaponTrace" :TraceProfile "(Name=\"NoCollision\")" :StartLocation (Utilities|Struct|MakeGameplayAbilityTargetingLocationInfo "LiteralTransform" "0.000000,0.000000,0.000000|0.000000,0.000000,-0.000000|1.000000,1.000000,1.000000" (Ability|GetAvatarActorfromActorInfo)) :ReticleClass 0)
      (:ValidData
        (CallFunction|Fire _data _bislast)
        (Utilities|FlowControl|Delay 0.08)
        (Ability|EndAbility))
      (:Cancelled
        (Ability|CancelAbility)))
    (else
      (Ability|Tasks|WaitInputRelease false
        (:OnRelease
          (Ability|CancelAbility))))))

(fn Fire
  (params (Data :type Gameplay%20Ability%20Target%20Data%20Handle%20Structure) (IsLast :type Boolean))
  (bind _returnvalue (Ability|TargetData|GetHitResultfromTargetData Data))
  (bind _as_bp_player_character (Variables|Default|GetAs%20BP%20Player%20Character))
  (bind (_bblockinghit _binitialoverlap _time _distance _location _impactpoint _normal _impactnormal _physmat _hitactor _hitcomponent _hitbonename _bonename _hititem _elementindex _faceindex _tracestart _traceend) (Collision|BreakHitResult _returnvalue))
  (bind _viewweaponmesh (Variables|/Script/NL_GAS.NLPlayerCharacter|GetViewWeaponMesh _as_bp_player_character))
  (bind _returnvalue_2 (Transformation|GetSocketLocation _viewweaponmesh "gun_muzzle_bulletEffect"))
  (LocalVariables|SetBulletStart _tracestart)
  (LocalVariables|SetBulletDirection (Math|Vector|Normalize (- (Math|Vector|SelectVector _impactpoint _traceend _bblockinghit) (LocalVariables|GetBulletStart))))
  (Utilities|FlowControl|Sequence
    (:then_0
      (Class|PlayerInterface|PlayCurrentWeaponMontage(Message) (Ability|GetAvatarActorfromActorInfo) (select (Class|NLPlayerCharacter|IsADS (Variables|Default|GetAs%20BP%20Player%20Character)) (GameplayTags|MakeLiteralGameplayTag "(TagName=\"Montage.Weapon.FireADS\")") (GameplayTags|MakeLiteralGameplayTag "(TagName=\"Montage.Weapon.Primary\")")))
      (if IsLast
        (Class|PlayerInterface|PlayCurrentWeaponMontage(Message) (Ability|GetAvatarActorfromActorInfo) (GameplayTags|MakeLiteralGameplayTag "(TagName=\"Montage.Weapon.LastFire\")"))))
    (:then_1
      (Ability|HasAuthority
        (:True
          (Game|SpawnActorfromClass "/Game/Blueprints/AbilitySystem/Abilities/Test/BP_TestProjectile.BP_TestProjectile_C" (Math|Transform|MakeTransform (+ (* (LocalVariables|GetBulletDirection) 2e+01) (LocalVariables|GetBulletStart)) (Math|Rotator|MakeRotfromX (LocalVariables|GetBulletDirection))) "AlwaysSpawn" "MultiplyWithRoot" (Ability|GetAvatarActorfromActorInfo) 0))
        (:False
          (Utilities|FlowControl|Sequence
            (:then_0
              (Class|PlayerInterface|WeaponFired(Message) (Ability|GetAvatarActorfromActorInfo) "/Game/Blueprints/CameraShake/Weapon/Rifle/CS_WeaponPrimary_SniperTEMP.CS_WeaponPrimary_SniperTEMP_C"))
            (:then_1
              (LocalVariables|SetNiagaraDirection (Math|Vector|Normalize (- (+ (* (LocalVariables|GetBulletDirection) 1e+03) (LocalVariables|GetBulletStart)) _returnvalue_2))))
            (:then_2
              (bind _returnvalue_3 (Niagara|SpawnSystematLocation "/Game/Assets/FX/NS_BulletTrail_View.NS_BulletTrail_View" _returnvalue_2))
              (Effects|Components|ParticleSystem|SetVectorParameter _returnvalue_3 "Direction" (LocalVariables|GetNiagaraDirection)))
            (:then_3
              (bind _returnvalue_4 (Niagara|SpawnSystematLocation "/Game/Assets/FX/NS_MuzzleSmoke.NS_MuzzleSmoke" (Transformation|GetSocketLocation (Variables|/Script/NL_GAS.NLPlayerCharacter|GetViewWeaponMesh (Variables|Default|GetAs%20BP%20Player%20Character)) "gun_muzzle")))
              (Effects|Components|ParticleSystem|SetVectorParameter _returnvalue_4 "Direction" (LocalVariables|GetNiagaraDirection)))))))))