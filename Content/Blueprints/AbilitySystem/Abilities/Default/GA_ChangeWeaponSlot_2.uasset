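; Gameplay ability that switches the player character to the second weapon slot.
; On activation it casts the avatar to BP_PlayerCharacter and calls ChangeWeaponSlotSimple with index 1 on its NLPlayerComponent.
; It then prints the current slot as debug output and ends immediately, with a second debug print on end.
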(event Ability|EventActivateAbility
  (Utilities|FlowControl|Sequence
    (:then_0
      (bind _asbp_player_character (Utilities|Casting|CastToBP_PlayerCharacter (Ability|GetAvatarActorfromActorInfo)))
      (Class|NLPlayerComponent|ChangeWeaponSlotSimple (Variables|/Script/NL_GAS.NLPlayerCharacter|GetNLPlayerComponent _asbp_player_character) 1)
      (Development|PrintString (Utilities|String|Append "Selected Weapon Slot: " (Utilities|String|ToString(Integer) (Math|Conversions|ToInteger(Byte) (Variables|/Script/NL_GAS.NLPlayerComponent|GetCurrentWeaponSlot (Variables|/Script/NL_GAS.NLPlayerCharacter|GetNLPlayerComponent _asbp_player_character))))))
      (Ability|EndAbility))))

(event Ability|EventOnEndAbility
  (params (bWasCancelled :type Boolean))
  (Development|PrintString "End"))