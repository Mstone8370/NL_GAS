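; Gameplay ability that switches the player to the first weapon slot.
; On activation it casts the avatar to Character, gets its BP_NLPlayerState and calls ChangeWeaponSlot with index 0.
; It then prints the selected slot for debugging and ends immediately; a failed cast stops before EndAbility is reached.
; Montage playback and gameplay-event wait nodes are present but disconnected, so they never run.
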(event Ability|EventActivateAbility
  (Utilities|FlowControl|Sequence
    (:then_0
      (bind _as캐릭터 (Utilities|Casting|CastToCharacter (Ability|GetAvatarActorfromActorInfo)))
      (bind _asbp_nlplayer_state (Utilities|Casting|CastToBP_NLPlayerState (Variables|/Script/Engine.Pawn|GetPlayerState _as캐릭터)))
      (Class|NLPlayerState|ChangeWeaponSlot _asbp_nlplayer_state)
      (Development|PrintString (Utilities|String|Append "Selected Weapon Slot: " (Utilities|String|ToString(Integer) (Math|Conversions|ToInteger(Byte) (Variables|/Script/NL_GAS.NLPlayerState|GetCurrentWeaponSlot _asbp_nlplayer_state)))))
      (Ability|EndAbility))))

(event Ability|EventOnEndAbility
  (params (bWasCancelled :type Boolean))
  (Development|PrintString "End"))