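; Base Gameplay Ability for swapping the avatar actor to the weapon slot given by SlotNum.
; Activation sends a TrySwapWeaponSlot interface message to the avatar with SlotNum minus one as the index, then ends the ability immediately.
; CanActivateAbility asks the avatar through CanSwapWeaponSlot with the same index, so the avatar owns both the validation and the swap logic.
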(event Ability|EventActivateAbility
  (Class|PlayerInterface|TrySwapWeaponSlot(Message) (Ability|GetAvatarActorfromActorInfo) (- (Variables|Default|GetSlotNum) 1))
  (Ability|EndAbility))

(event Ability|EventOnEndAbility
  (params (bWasCancelled :type Boolean)))

(fn K2CanActivateAbility
  (params (ActorInfo :type Gameplay%20Ability%20Actor%20Info%20Structure) (Handle :type Gameplay%20Ability%20Spec%20Handle%20Structure))
  (bind _returnvalue (Class|PlayerInterface|CanSwapWeaponSlot(Message) (.AvatarActor (Utilities|Struct|BreakGameplayAbilityActorInfo ActorInfo)) (- (Variables|Default|GetSlotNum) 1)))
  (return "" _returnvalue))