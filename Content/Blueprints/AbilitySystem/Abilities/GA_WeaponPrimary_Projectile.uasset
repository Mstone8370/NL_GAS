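; Primary weapon gameplay ability that fires a projectile and plays its muzzle effects.
; Fire derives bullet start and direction from a hit result, aiming at the impact point or trace end, and spawns BP_TestProjectile on authority.
; SpawnFX gets weapon socket locations from the avatar and spawns Niagara trail and muzzle smoke, both angled from the effect socket toward a point along the bullet path.
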(event Ability|EventActivateAbility
  (|CallParentFunction) ; 지금 이 노드는 비활성 상태입니다. \n핀을 끌어서 다른 노드를 연결하면 활성화됩니다.
)

(fn Fire
  (params (HitResult :type Hit%20Result%20Structure))
  (bind (_bblockinghit _binitialoverlap _time _distance _location _impactpoint _normal _impactnormal _physmat _hitactor _hitcomponent _hitbonename _bonename _hititem _elementindex _faceindex _tracestart _traceend) (Collision|BreakHitResult HitResult))
  (Utilities|FlowControl|Sequence
    (:then_0
      (Variables|Default|SetBulletStart _tracestart)
      (Variables|Default|SetBulletEnd (Math|Vector|SelectVector _impactpoint _traceend _bblockinghit))
      (Variables|Default|SetBulletDirection (Math|Vector|Normalize (- (Variables|Default|GetBulletEnd) (Variables|Default|GetBulletStart)))))
    (:then_1
      (Ability|HasAuthority
        (:True
          (Game|SpawnActorfromClass "/Game/Blueprints/AbilitySystem/Abilities/Test/BP_TestProjectile.BP_TestProjectile_C" (Math|Transform|MakeTransform (+ (* (Variables|Default|GetBulletDirection) 1.0) (Variables|Default|GetBulletStart)) (Math|Rotator|MakeRotfromX (Variables|Default|GetBulletDirection))) "AlwaysSpawn" "MultiplyWithRoot" (Ability|GetAvatarActorfromActorInfo) 0))))))

(fn SpawnFX
  (params (TargetDataHitResult :type Hit%20Result%20Structure))
  (bind (_outleftiklocation _outrightiklocation) (Class|PlayerInterface|GetWeaponHandIKLocation(Message) (Ability|GetAvatarActorfromActorInfo) "gun_muzzle_bulletEffect" "gun_muzzle"))
  (Utilities|FlowControl|Sequence
    (:then_0
      (LocalVariables|SetNiagaraDirection (Math|Vector|Normalize (- (+ (* (Variables|Default|GetBulletDirection) 1e+03) (Variables|Default|GetBulletStart)) _outleftiklocation))))
    (:then_1
      (bind _returnvalue (Niagara|SpawnSystematLocation "/Game/Assets/FX/NS_BulletTrail_View.NS_BulletTrail_View" _outleftiklocation))
      (Effects|Components|ParticleSystem|SetVectorParameter _returnvalue "Direction" (LocalVariables|GetNiagaraDirection)))
    (:then_2
      (bind _returnvalue_2 (Niagara|SpawnSystematLocation "/Game/Assets/FX/NS_MuzzleSmoke.NS_MuzzleSmoke" _outrightiklocation))
      (Effects|Components|ParticleSystem|SetVectorParameter _returnvalue_2 "Direction" (LocalVariables|GetNiagaraDirection)))))